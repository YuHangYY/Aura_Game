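; GA_Electrocute is Aura's held-input lightning beam ability, handling animation, movement lock and beam visuals.
; On activation it stores cursor hit data, hides the cursor, faces the target and plays the montage.
; The montage's gameplay event starts the shock loop, disables movement, traces the first target and adds the ShockLoop cue to it, or to the caster if it lacks CombatInterface.
; Input release restores cursor and movement, removes the cue and ends the ability.
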(event Ability|EventActivateAbility
  (CallFunction|检测此角色是否继承了Combat接口)
  ;[1 1 1] 存储鼠标检测数据和控制器数据
  (bind _datahandle (|TargetDataUnderMouse)
    (:DataValid
      (Class|AuraBeamSpell|StoreMouseDataInfo (Ability|TargetData|GetHitResultfromTargetData _datahandle))
      (Class|AuraBeamSpell|StoreOwingPlayerController)
      (Utilities|FlowControl|Sequence
        (:then_0
          (Variables|/Script/Engine.PlayerController|SetbShowMouseCursor (Variables|Default|GetOwningPlayerController) false)
          (Class|CombatInterface|UpdateFacingTarget(Message) (Ability|GetAvatarActorfromActorInfo) (Variables|Default|GetMouseHitLocation))
          (GameplayCue|ExecuteGameplayCue :GameplayCueTag "(TagName=\"GameplayCue.ShockBrust\")")
          (|PlayMontageandWaitProxy "None" (Variables|Default|GetMontage_Electrocute) 1.0 "None" true 1.0 0.0 false
            (:then
              (Ability|Tasks|WaitGameplayEvent "(TagName=\"Event.Montage.Electrocute\")" 0
                (:EventReceived
                  (CallFunction|开始电击动作)
                  (CallFunction|生成电光束))))))
        (:then_1
          (Ability|Tasks|WaitInputRelease false
            (:OnRelease
              (CallFunction|电击结束)
              (Ability|EndAbility))))))))

(fn 检测此角色是否继承了Combat接口
  (if (not (Utilities|DoesObjectImplementInterface (Ability|GetAvatarActorfromActorInfo) "/Script/Aura_Game.CombatInterface"))
    (Ability|EndAbility)))

(fn 开始电击动作
  (Class|CombatInterface|SetIsShockLoop(Message) (Ability|GetAvatarActorfromActorInfo) true)
  (Pawn|Components|CharacterMovement|DisableMovement (Variables|/Script/Engine.Character|GetCharacterMovement (Variables|Default|GetOwnerCharacter))))

(fn 电击结束
  (Variables|/Script/Engine.PlayerController|SetbShowMouseCursor (Variables|Default|GetOwningPlayerController) true)
  (Class|CombatInterface|SetIsShockLoop(Message) (Ability|GetAvatarActorfromActorInfo) false)
  (Pawn|Components|CharacterMovement|SetMovementMode (Variables|/Script/Engine.Character|GetCharacterMovement (Variables|Default|GetOwnerCharacter)) "MOVE_Walking" 0)
  (if (Variables|Default|GetIsImplementInterface)
    (GameplayCue|RemoveGameplayCueOnActor(Looping) (Variables|Default|GetTargetActor) "(TagName=\"GameplayCue.ShockLoop\")" (Variables|Default|GetTraceFirstResult))
    (else
      (GameplayCue|RemoveGameplayCueOnActor(Looping) (Ability|GetAvatarActorfromActorInfo) "(TagName=\"GameplayCue.ShockLoop\")" (Variables|Default|GetTraceFirstResult)))))

(fn 生成电光束
  (Class|AuraBeamSpell|TraceFirstTarget (Variables|Default|GetMouseHitLocation))
  (bind _returnvalue (Class|CombatInterface|GetWeaponComponent(Message) (Ability|GetAvatarActorfromActorInfo)))
  (Variables|Default|SetTraceFirstResult (Ability|GameplayCue|MakeGameplayCueParameters :Location (Variables|Default|GetMouseHitLocation) :SourceObject (Variables|Default|GetHitActor) :TargetAttachComponent _returnvalue))
  ;[1 0.8707 0.2011] 被鼠标击中的角色是敌人吗？
  (bind _output_get (Variables|Default|SetIsImplementInterface (Utilities|DoesObjectImplementInterface (Variables|Default|GetHitActor) "/Script/Aura_Game.CombatInterface")))
  (if _output_get
    (Variables|Default|SetTargetActor (Variables|Default|GetHitActor))
    (else
      (Variables|Default|SetTargetActor (Ability|GetAvatarActorfromActorInfo))))
  (GameplayCue|AddGameplayCueOnActor(Looping) (Variables|Default|GetTargetActor) "(TagName=\"GameplayCue.ShockLoop\")" (Variables|Default|GetTraceFirstResult)))