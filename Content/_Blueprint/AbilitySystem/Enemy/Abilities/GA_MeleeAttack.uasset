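; GA_MeleeAttack is an enemy gameplay ability that performs a melee attack with a randomly chosen montage.
; It turns the avatar toward its combat target, plays the montage and waits for that montage's gameplay event.
; On the event, it gathers living actors near the tagged weapon socket and damages those passing the ISBothFirend check.
; Any hit triggers a MeleeEffect gameplay cue at the weapon location, then the ability ends.
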(event Ability|EventActivateAbility
  (bind _returnvalue (Ability|GetAvatarActorfromActorInfo))
  (bind _returnvalue_2 (Ability|GetAvatarActorfromActorInfo))
  (bind _ascombat_interface (Utilities|Casting|CastToCombatInterface _returnvalue))
  (bind _returnvalue_3 (Class|EnemyInterface|GetCombatTarget(Message) _returnvalue))
  (Class|CombatInterface|UpdateFacingTarget _ascombat_interface (Transformation|GetActorLocation _returnvalue_3))
  (bind _returnvalue_4 (Class|CombatInterface|GetAttackAnimMontage(Message) (Ability|GetAvatarActorfromActorInfo)))
  (bind _returnvalue_5 (Class|AuraDamageGameplayAbility|GetRandomAttackMontagefromArray _returnvalue_4))
  (bind _output_get (Variables|Default|SetAttackMontageArray _returnvalue_5))
  (|PlayMontageandWaitProxy "None" (.AttackMontage (Utilities|Struct|BreakTaggedMontage _output_get)) 1.0 "None" false 1.0 0.0 false
    (:then
      (Ability|Tasks|WaitGameplayEvent (.MontageTag (Utilities|Struct|BreakTaggedMontage _output_get)) 0
        (:EventReceived
          (bind _returnvalue_6 (Class|CombatInterface|GetCombaWeaponLocation(Message) _returnvalue_2 (.SocketTag (Utilities|Struct|BreakTaggedMontage _output_get))))
          (Variables|Default|SetWeaponLocation _returnvalue_6)
          (bind _outactors (Class|AuraWidgetControllerLibrary|GetLifeActorWithingRadius _returnvalue_2 (Utilities|Array|MakeArray _returnvalue_2) 6e+01 (Variables|Default|GetWeaponLocation)))
          (for _array_element _outactors
            (bind _returnvalue_7 (Class|AuraWidgetControllerLibrary|ISBothFirend (Ability|GetAvatarActorfromActorInfo) _array_element))
            (if _returnvalue_7
              (Variables|Default|SetHasHitTarget true)
              (Class|AuraDamageGameplayAbility|CauseDamage _array_element)))
          (if (Variables|Default|GetHasHitTarget)
            (Class|GameplayAbility|ExecuteGameplayCuewithParams "(TagName=\"GameplayCue.MeleeEffect\")" (Ability|GameplayCue|MakeGameplayCueParameters :AggregatedSourceTags (GameplayTags|MakeGameplayTagContainerfromTag (.MontageTag (Utilities|Struct|BreakTaggedMontage (Variables|Default|GetAttackMontageArray)))) :Location (Variables|Default|GetWeaponLocation) :EffectCauser (Ability|GetAvatarActorfromActorInfo))))
          (Ability|EndAbility))))))

(event Ability|EventOnEndAbility
  (params (bWasCancelled :type Boolean)))