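; Enemy ranged attack Gameplay Ability that turns the avatar toward its combat target and fires a projectile at it.
; It plays a random attack montage from the avatar's list and starts a gameplay event wait on a montage tag from a separate random pick.
; The projectile spawns from the wait task's immediate Then output, not the received event, and the ability ends after a short delay, or immediately without montages.
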(event Ability|EventActivateAbility
  (bind _returnvalue (Ability|GetAvatarActorfromActorInfo))
  (bind _returnvalue_2 (Class|EnemyInterface|GetCombatTarget(Message) _returnvalue))
  (Class|CombatInterface|UpdateFacingTarget(Message) _returnvalue (Transformation|GetActorLocation _returnvalue_2))
  (bind _returnvalue_3 (Class|CombatInterface|GetAttackAnimMontage(Message) (Ability|GetAvatarActorfromActorInfo)))
  (if (> (Utilities|Array|Length _returnvalue_3) 0)
    (|PlayMontageandWaitProxy "None" (.AttackMontage (Utilities|Struct|BreakTaggedMontage (Utilities|Array|Get(acopy) _returnvalue_3 (Math|Random|RandomIntegerinRange 0 (- (Utilities|Array|Length _returnvalue_3) 1))))) 1.0 "None" true 1.0 0.0 false
      (:then
        (Ability|Tasks|WaitGameplayEvent (.MontageTag (Utilities|Struct|BreakTaggedMontage (Utilities|Array|Get(acopy) _returnvalue_3 (Math|Random|RandomIntegerinRange 0 (- (Utilities|Array|Length _returnvalue_3) 1))))) 0
          (:then
            (bind _returnvalue_4 (Class|EnemyInterface|GetCombatTarget(Message) (Ability|GetAvatarActorfromActorInfo)))
            (Class|AuraProjectileSpell|SpawnProjectile (Transformation|GetActorLocation _returnvalue_4))
            (Utilities|FlowControl|Delay 0.5)
            (Ability|EndAbility)))))
    (else
      (Ability|EndAbility))))

(event Ability|EventOnEndAbility
  (params (bWasCancelled :type Boolean)))